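; BP_ToSpawn is a pickup-style actor with two text labels that reacts when the player comes near.
; Tick polls the distance to player pawn 0; within a short range it plays a pickup sound, spawns a particle effect above itself, hides both labels and sets a Lock flag.
; Once locked, Tick accumulates time and, after a brief delay, CleanUp destroys the particle component and the actor.
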(event Custom|CleanUp
  (bind _particles (Variables|Default|GetParticleS))
  (Utilities|IsValid _particles
    (:Is%20Valid
      (Components|DestroyComponent _particles))
    (:Is%20Not%20Valid
      _))
  (Actor|DestroyActor))

(event EventBeginPlay)

(event Collision|EventActorBeginOverlap
  (params (OtherActor :type Actor%20Object%20Reference)))

(event EventTick
  (params (DeltaSeconds :type Float%20%28single-precision%29))
  (bind _returnvalue (Game|Player|GetPlayerPawn 0))
  (bind _returnvalue_2 (Transformation|GetActorLocation))
  (bind _returnvalue_3 (Transformation|GetActorUpVector))
  (bind _returnvalue_4 (* _returnvalue_3 1e+02))
  (bind _returnvalue_5 (+ _returnvalue_2 _returnvalue_4))
  (if (not (Variables|Default|GetLock))
    (Utilities|IsValid _returnvalue
      (:Is%20Valid
        (if (< (Math|Vector|VectorLength (- _returnvalue_2 (Transformation|GetActorLocation _returnvalue))) 2.5e+02)
          (Audio|PlaySoundatLocation "/Engine/VREditor/Sounds/UI/Object_PickUp.Object_PickUp" _returnvalue_5 "0, 0, 0" 1.0 1.0 0.0 0 0 0)
          (bind _returnvalue_6 (Effects|SpawnEmitteratLocation "/Engine/Tutorial/SubEditors/TutorialAssets/TutorialParticleSystem.TutorialParticleSystem" _returnvalue_5 (Transformation|GetActorRotation)))
          (Variables|Default|SetParticleS _returnvalue_6)
          (Variables|Default|SetLock true)
          (Rendering|SetVisibility (Variables|Default|GetTextRender) false false)
          (Rendering|SetVisibility (Variables|Default|GetTextRender1) false false))))
    (else
      (bind _output_get (Variables|Default|SetTimeAc (+ (Variables|Default|GetTimeAc) DeltaSeconds)))
      (if (> _output_get 2.0)
        (CallFunction|CleanUp)))))

(fn ConstructionScript)